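; Base NPC that registers with the third-person game mode's NPC count on spawn and can die from damage or being run over.
; Damage lowers Health; a hit once it is depleted calls Consume on the first BP_Character found, decrements the count and destroys the NPC.
; A run-over by a fast-moving character ragdolls it without capsule collision, then after a delay decrements and destroys it without Consume.
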(event `self.ReceiveBeginPlay`
  (`self.OnSpawn`))

(event `self.ReceiveAnyDamage`
  (params (Damage :type "Float (single-precision)") (DamageType :type "DamageType Object Reference") (InstigatedBy :type "Controller Object Reference") (DamageCauser :type "Actor Object Reference"))
  (if (> (`self.Health`) 0.0)
    (set `self.Health` (- (`self.Health`) Damage))
    (`KismetSystemLibrary.PrintString` "Damage Recived")
    (elif (not (`self.RunOverDeath`))
      (`self.ConsumeDeath`))))

(event `/Game/BluePrints/NPCS/1/OnRunOver.OnRunOver`
  (params (Character :type "Actor Object Reference"))
  (if (> (`KismetMathLibrary.VSizeXY` (`self.GetVelocity` Character)) 500.0)
    (`PrimitiveComponent.SetSimulatePhysics` (`self.Mesh`) true)
    (`PrimitiveComponent.SetCollisionEnabled` (`self.CapsuleComponent`) "NoCollision")
    (`KismetSystemLibrary.Delay` 2.0)
    (`self.Death`)
    (set `self.RunOverDeath` true)))

(fn `ConsumeDeath`
  (bind _outactors (`GameplayStatics.GetAllActorsOfClass` "/Game/BluePrints/BP_Character.BP_Character_C"))
  (for _array_element _outactors
    (`/Game/BluePrints/BP_Character.Consume` _array_element)
    (bind _asbp_third_person_game_mode (cast `/Game/ThirdPerson/Blueprints/BP_ThirdPersonGameMode` (`GameplayStatics.GetGameMode`)))
    (`/Game/ThirdPerson/Blueprints/BP_ThirdPersonGameMode.DecreaseNPC` _asbp_third_person_game_mode)
    (`self.K2_DestroyActor`)
    (return)))

(fn `Death`
  (bind _asbp_third_person_game_mode (cast `/Game/ThirdPerson/Blueprints/BP_ThirdPersonGameMode` (`GameplayStatics.GetGameMode`)))
  (`/Game/ThirdPerson/Blueprints/BP_ThirdPersonGameMode.DecreaseNPC` _asbp_third_person_game_mode)
  (`self.K2_DestroyActor`)
  (return))

(fn `OnSpawn`
  (bind _asbp_third_person_game_mode (cast `/Game/ThirdPerson/Blueprints/BP_ThirdPersonGameMode` (`GameplayStatics.GetGameMode`)))
  (`/Game/ThirdPerson/Blueprints/BP_ThirdPersonGameMode.IncreaseNPC` _asbp_third_person_game_mode)
  (return))

(fn `UserConstructionScript`)