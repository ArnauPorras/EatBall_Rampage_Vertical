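; BP_NPC_Spawner keeps the level populated with NPCs of a configurable class, spawning them in batches at random reachable navmesh points around itself.
; BeginPlay spawns the first batch immediately, then caches BP_ThirdPersonGameMode.
; After a short random delay, it spawns another full batch if the game mode's NPCAlive is below MaxAlive.
; Otherwise, ShouldSpawn keeps polling on similar delays until room opens up.
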(event `self.ReceiveBeginPlay`
  (`|ExecutionSequence`
    (:`then_0`
      (`self.NPC_Spawn` (`self.Number Of Enemies`) (`self.Class`)))
    (:`then_1`
      (bind _asbp_third_person_game_mode (cast `/Game/ThirdPerson/Blueprints/BP_ThirdPersonGameMode` (`GameplayStatics.GetGameMode`)))
      (set `self.As BP Third Person Game Mode` _asbp_third_person_game_mode))))

(event `NPC_Spawn`
  (params (NumberOfEnemies :type Integer) (Class :type "Actor Class Reference"))
  (bind _as_bp_third_person_game_mode (`self.As BP Third Person Game Mode`))
  (for _ (range NumberOfEnemies)
    (`|SpawnActorFromClass` Class (`KismetMathLibrary.MakeTransform` (`NavigationSystemV1.K2_GetRandomReachablePointInRadius` (`self.K2_GetActorLocation` self) 7000.0 null null)) "Undefined" "MultiplyWithRoot" null null))
  (`KismetSystemLibrary.Delay` (`KismetMathLibrary.RandomFloatInRange` 0.5 1.0))
  (if (< (`/Game/ThirdPerson/Blueprints/BP_ThirdPersonGameMode.NPCAlive` _as_bp_third_person_game_mode) (`/Game/ThirdPerson/Blueprints/BP_ThirdPersonGameMode.MaxAlive` _as_bp_third_person_game_mode))
    (`self.NPC_Spawn` (`self.Number Of Enemies`) (`self.Class`))
    (else
      (`self.ShouldSpawn`))))

(event `ShouldSpawn`
  (bind _as_bp_third_person_game_mode (`self.As BP Third Person Game Mode`))
  (`KismetSystemLibrary.Delay` (`KismetMathLibrary.RandomFloatInRange` 0.5 1.0))
  (if (< (`/Game/ThirdPerson/Blueprints/BP_ThirdPersonGameMode.NPCAlive` _as_bp_third_person_game_mode) (`/Game/ThirdPerson/Blueprints/BP_ThirdPersonGameMode.MaxAlive` _as_bp_third_person_game_mode))
    (`self.NPC_Spawn` (`self.Number Of Enemies`) (`self.Class`))
    (else
      (`self.ShouldSpawn`))))

(fn `UserConstructionScript`)