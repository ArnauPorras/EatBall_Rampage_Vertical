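; TestCube is a damageable test actor that feeds player growth by calling Consume on BP_Character actors when it dies.
; AnyDamage subtracts from Health and prints a message while Health is positive.
; A hit arriving at zero or less calls Consume on every BP_Character, destroying the cube inside that loop.
; Unconnected leftover nodes would scale capsule, camera boom, bite area and damage, and lower rotation speed.
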(event `self.ReceiveAnyDamage`
  (params (Damage :type "Float (single-precision)") (DamageType :type "DamageType Object Reference") (InstigatedBy :type "Controller Object Reference") (DamageCauser :type "Actor Object Reference"))
  (if (> (`self.Health`) 0.0)
    (set `self.Health` (- (`self.Health`) Damage))
    (`KismetSystemLibrary.PrintString` "Damage Recived")
    (else
      (bind _outactors (`GameplayStatics.GetAllActorsOfClass` "/Game/BluePrints/BP_Character.BP_Character_C"))
      (for _array_element _outactors
        (`/Game/BluePrints/BP_Character.Consume` _array_element)
        (`self.K2_DestroyActor`)))))

(fn `UserConstructionScript`)